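; Player stats component for BP_ThirdPersonCharacter that tracks health, stamina, XP and level and pushes changes to the HUD.
; BeginPlay waits a tick, caches the owning character, then fills the health and stamina bars and level text.
; Increase functions cap current values at max, while decrease functions return true once depleted.
; XP overflow carries into a level-up, which raises the XP threshold, updates the HUD and plays a sound.
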(event `self.ReceiveBeginPlay`
  (`KismetSystemLibrary.DelayUntilNextTick`)
  (bind _asbp_third_person_character (cast `/Game/ThirdPerson/Blueprints/BP_ThirdPersonCharacter` (`self.GetOwner`)))
  (set `self.PlayerCharacterBP` _asbp_third_person_character)
  ;[0.05127 0.05127 0.05127] Sets percentages for Health and Stamina Bar
  (`ProgressBar.SetPercent` (`/Game/UI/WB_HUD.HealthBar` (`/Game/ThirdPerson/Blueprints/BP_ThirdPersonCharacter.HUD Widget` (`self.PlayerCharacterBP`))) (/ (`self.CurrentHealth`) (`self.MaxHealth`)))
  (`ProgressBar.SetPercent` (`/Game/UI/WB_HUD.StaminaBar` (`/Game/ThirdPerson/Blueprints/BP_ThirdPersonCharacter.HUD Widget` (`self.PlayerCharacterBP`))) (/ (`self.CurrentStamina`) (`self.MaxStamina`)))
  ;[0.05127 0.05127 0.05127] Show Level on HUD
  (`TextBlock.SetText` (`/Game/UI/WB_HUD.LevelNum` (`/Game/ThirdPerson/Blueprints/BP_ThirdPersonCharacter.HUD Widget` (`self.PlayerCharacterBP`))) (`KismetTextLibrary.Conv_IntToText` (`self.Level`))))

(fn `DecreaseHealth`
  (params (Damage :type "Float (double-precision)"))
  (returns (`Is Player Dead?` :type Boolean))
  ;[0.05127 0.05127 0.05127] Checks that we can decrease health
  (if (not (<= (`self.CurrentHealth`) 0.0))
    ;[0.05127 0.05127 0.05127] Updates Health bar
    (bind _output_get (set `self.CurrentHealth` (- (`self.CurrentHealth`) Damage)))
    (`ProgressBar.SetPercent` (`/Game/UI/WB_HUD.HealthBar` (`/Game/ThirdPerson/Blueprints/BP_ThirdPersonCharacter.HUD Widget` (`self.PlayerCharacterBP`))) (/ _output_get (`self.MaxHealth`)))
    (if (<= (`self.CurrentHealth`) 0.0)
      _
      (else
        (return false))))
  (return true))

(fn `DecreaseStamina`
  (params (`Stamina Depleted` :type "Float (double-precision)"))
  (returns (`No Stamina?` :type Boolean))
  (if (not (<= (`self.CurrentStamina`) 0.0))
    (bind _output_get (set `self.CurrentStamina` (- (`self.CurrentStamina`) `Stamina Depleted`)))
    ;[0.05127 0.05127 0.05127] Updates Stamina Bar
    (`ProgressBar.SetPercent` (`/Game/UI/WB_HUD.StaminaBar` (`/Game/ThirdPerson/Blueprints/BP_ThirdPersonCharacter.HUD Widget` (`self.PlayerCharacterBP`))) (/ _output_get (`self.MaxStamina`)))
    (if (<= (`self.CurrentStamina`) 0.0)
      _
      (else
        (return false))))
  (return true))

(fn `IncreaseHealth`
  (params (`Added Health` :type "Float (double-precision)"))
  (bind _output_get (set `self.CurrentHealth` (+ (`self.CurrentHealth`) `Added Health`)))
  (if (> _output_get (`self.MaxHealth`))
    (bind _output_get_2 (set `self.CurrentHealth` (`self.MaxHealth`))))
  ;[0.05127 0.05127 0.05127] Updates Health Bar
  (`ProgressBar.SetPercent` (`/Game/UI/WB_HUD.HealthBar` (`/Game/ThirdPerson/Blueprints/BP_ThirdPersonCharacter.HUD Widget` (`self.PlayerCharacterBP`))) (/ _output_get_2 (`self.MaxHealth`))))

(fn `IncreaseLevel`
  (set `self.Level` (+ (`self.Level`) 1))
  ;[0.05127 0.05127 0.05127] Increase Maximum XP
  (set `self.MaxXP` (+ (`self.MaxXP`) 150.0))
  ;[0.05127 0.05127 0.05127] Show Level on HUD
  (`TextBlock.SetText` (`/Game/UI/WB_HUD.LevelNum` (`/Game/ThirdPerson/Blueprints/BP_ThirdPersonCharacter.HUD Widget` (`self.PlayerCharacterBP`))) (`KismetTextLibrary.Conv_IntToText` (`self.Level`)))
  (`GameplayStatics.PlaySound2D` "/Game/Audio/UI/LevelUp.LevelUp" 1.0 1.0 0.0 null null))

(fn `IncreaseMaxHealth`
  (params (`Max Health Increase` :type "Float (double-precision)"))
  (set `self.MaxHealth` (+ (`self.MaxHealth`) `Max Health Increase`))
  ;[0.05127 0.05127 0.05127] Updates Health Bar
  (`ProgressBar.SetPercent` (`/Game/UI/WB_HUD.HealthBar` (`/Game/ThirdPerson/Blueprints/BP_ThirdPersonCharacter.HUD Widget` (`self.PlayerCharacterBP`))) (/ (`self.CurrentHealth`) (`self.MaxHealth`))))

(fn `IncreaseMaxStamina`
  (params (`Added Stamina` :type "Float (double-precision)"))
  (bind _output_get (set `self.MaxStamina` (+ (`self.MaxStamina`) `Added Stamina`)))
  ;[0.05127 0.05127 0.05127] Updates Stamina Bar
  (`ProgressBar.SetPercent` (`/Game/UI/WB_HUD.StaminaBar` (`/Game/ThirdPerson/Blueprints/BP_ThirdPersonCharacter.HUD Widget` (`self.PlayerCharacterBP`))) (/ (`self.CurrentStamina`) _output_get)))

(fn `IncreaseStamina`
  (params (`Added Stamina` :type "Float (double-precision)"))
  (bind _output_get (set `self.CurrentStamina` (+ `Added Stamina` (`self.CurrentStamina`))))
  (if (> _output_get (`self.MaxStamina`))
    (bind _output_get_2 (set `self.CurrentStamina` (`self.MaxStamina`))))
  ;[0.05127 0.05127 0.05127] Updates Stamina Bar
  (`ProgressBar.SetPercent` (`/Game/UI/WB_HUD.StaminaBar` (`/Game/ThirdPerson/Blueprints/BP_ThirdPersonCharacter.HUD Widget` (`self.PlayerCharacterBP`))) (/ _output_get_2 (`self.MaxStamina`))))

(fn `IncreaseXP`
  (params (`Added XP` :type "Float (double-precision)"))
  (bind _output_get (set `self.XP` (+ (`self.XP`) `Added XP`)))
  (if (>= _output_get (`self.MaxXP`))
    (set `self.XP` (- (`self.XP`) (`self.MaxXP`)))
    (`self.IncreaseLevel`)))