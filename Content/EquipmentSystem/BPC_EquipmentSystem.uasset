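; Actor component on the third-person character that handles picking up weapons and toggling the equipment menu.
; Interact runs a debug-drawn sphere trace from the follow camera; a hit BP_Weapon has its ItemData added to WeaponSlots and is destroyed.
; The menu input shows or hides a reused WB_Equipment widget, switches cursor and input mode, disables or restores movement, and near-freezes time through global time dilation.
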(event `self.ReceiveBeginPlay`
  (bind _asbp_third_person_character (cast `/Game/ThirdPerson/Blueprints/BP_ThirdPersonCharacter` (`self.GetOwner`)))
  (set `self.Follow Camera` (`/Game/ThirdPerson/Blueprints/BP_ThirdPersonCharacter.FollowCamera` _asbp_third_person_character)))

(event `EnhancedInput|/Game/ThirdPerson/Input/Actions/IA_Interact`
  (params (ActionValue :type Boolean) (ElapsedSeconds :type "Float (double-precision)") (TriggeredSeconds :type "Float (double-precision)") (InputAction :type "InputAction Object Reference" :default "/Game/ThirdPerson/Input/Actions/IA_Interact.IA_Interact"))
  (bind _follow_camera (`self.Follow Camera`))
  (bind _returnvalue (`SceneComponent.K2_GetComponentLocation` _follow_camera))
  ;[0.05127 0.05127 0.05127] Pick Up Item Trace
  (:`Started`
    (bind (_outhit _returnvalue_2) (`KismetSystemLibrary.SphereTraceSingleForObjects` :`Start` _returnvalue :`End` (+ _returnvalue (* (`KismetMathLibrary.GetForwardVector` (`SceneComponent.K2_GetComponentRotation` _follow_camera)) 750.0)) :`Radius` 100.0 :`ObjectTypes` (`|MakeArray` "ObjectTypeQuery2" :!type "EObjectTypeQuery Enum") :`DrawDebugType` "ForDuration"))
    (if _returnvalue_2
      (bind _asbp_weapon (cast `/Game/EquipmentSystem/BP_Weapon` (`.HitActor` (`GameplayStatics.BreakHitResult` _outhit))))
      (`self.AddWeapon` (`/Game/EquipmentSystem/BP_Weapon.ItemData` _asbp_weapon))
      (`Actor.K2_DestroyActor` _asbp_weapon)
      (`KismetSystemLibrary.PrintString` "Item Gathered!"))))

(event `EnhancedInput|/Game/ThirdPerson/Input/Actions/IA_EquipmentMenu`
  (params (ActionValue :type Boolean) (ElapsedSeconds :type "Float (double-precision)") (TriggeredSeconds :type "Float (double-precision)") (InputAction :type "InputAction Object Reference" :default "/Game/ThirdPerson/Input/Actions/IA_EquipmentMenu.IA_EquipmentMenu"))
  (bind _returnvalue (`GameplayStatics.GetPlayerController` 0))
  ;[0.05127 0.05127 0.05127] Show Equipment Menu Panel
  (:`Started`
    (if (not (`self.isPanelOpened?`))
      (set `self.isPanelOpened?` true)
      (bind _equipmentwidget (`self.EquipmentWidget`)
        (:`then`
          (`Widget.SetVisibility` _equipmentwidget "Visible"))
        (:`else`
          (bind _returnvalue_2 (`|CreateWidget` "/Game/EquipmentSystem/UI/WB_Equipment.WB_Equipment_C"))
          (bind _output_get (set `self.EquipmentWidget` _returnvalue_2))
          (`UserWidget.AddToViewport` _output_get 0)))
      (set `PlayerController.bShowMouseCursor` true _returnvalue)
      (`WidgetBlueprintLibrary.SetInputMode_GameAndUIEx` _returnvalue (`self.EquipmentWidget`))
      (bind _asbp_third_person_character (cast `/Game/ThirdPerson/Blueprints/BP_ThirdPersonCharacter` (`self.GetOwner`)))
      (`CharacterMovementComponent.SetMovementMode` (`Character.CharacterMovement` _asbp_third_person_character) "MOVE_None" 0)
      (`GameplayStatics.SetGlobalTimeDilation` 0.001)
      (else
        (set `self.isPanelOpened?` false)
        (bind _equipmentwidget_2 (`self.EquipmentWidget`)
          (:`then`
            (`Widget.SetVisibility` _equipmentwidget_2 "Hidden")
            (set `PlayerController.bShowMouseCursor` false _returnvalue)
            (`WidgetBlueprintLibrary.SetInputMode_GameOnly` _returnvalue)
            (bind _asbp_third_person_character_2 (cast `/Game/ThirdPerson/Blueprints/BP_ThirdPersonCharacter` (`self.GetOwner`)))
            (`CharacterMovementComponent.SetMovementMode` (`Character.CharacterMovement` _asbp_third_person_character_2) "MOVE_Walking" 0)
            (`GameplayStatics.SetGlobalTimeDilation` 1.0))
          (:`else`))))))

(fn `AddWeapon`
  (params (NewItem :type "/Game/EquipmentSystem/S_Slots Structure"))
  (`KismetArrayLibrary.Array_Add` (`self.WeaponSlots`) NewItem))